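; CloudRoot is a Blueprint that watches its scene root for movement, apparently intended to carry a set of cloud elements along with it.
; The construction script caches the root's world transform, and Tick compares against it, calling MoveThatThing on any change.
; MoveThatThing derives location and per-axis rotation deltas, then loops over Elements with an empty body, so nothing is moved yet.
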(event EventTick
  (params (DeltaSeconds :type Float%20%28single-precision%29))
  (bind _output_get (Variables|Default|SetCurTransform (Transformation|GetWorldTransform (Variables|Default|GetDefaultSceneRoot))))
  (if (not (== _output_get (Variables|Default|GetPrevTransform)))
    (CallFunction|MoveThatThing)
    (Variables|Default|SetPrevTransform (Variables|Default|GetCurTransform))))

(fn ConstructionScript
  (bind _output_get (Variables|Default|SetPrevTransform (Transformation|GetWorldTransform (Variables|Default|GetDefaultSceneRoot))))
  (Variables|Default|SetCurTransform _output_get))

(fn MoveThatThing
  (bind _curtransform (Variables|Default|GetCurTransform))
  (bind _prevtransform (Variables|Default|GetPrevTransform))
  (bind (_location _rotation) (Math|Transform|BreakTransform _prevtransform))
  (bind (_location_2 _rotation_2) (Math|Transform|BreakTransform _curtransform))
  (bind (_roll _pitch _yaw) (Math|Rotator|BreakRotator _rotation))
  (LocalVariables|SetDiffLoc (- _location_2 _location))
  (bind _result (CallFunction|RotatorAdd _rotation_2 (* -1 _roll) (* -1 _pitch) (* -1 _yaw)))
  (LocalVariables|SetDiffRot _result)
  (for _array_element (Variables|Default|GetElements)
    _))