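; CompParent is the parent Actor for modular building pieces that snap to six sides of one another.
; BuildingDispatcher either spawns a child at a free side's world-axis offset or sets Real/Stable/Constructed state.
; ReconstructClassObject destroys non-real pieces, or switches "Basement" mesh collision and material by Constructed, then retraces neighbors.
; RevalidateTrace line-traces from RootSphere to update neighbors and open sides; sides 1 and 3 both trace backward.
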(event `BuildingDispatcher`
  (params (CreateNew :type Boolean) (CollidingSide :type "ActorComponent Object Reference") (NewCompClass :type "Actor Class Reference") (SetReal :type Boolean) (SetStable :type Boolean) (SetConstructed :type Boolean))
  (if CreateNew
    (`self.ReconstructClassObject`)
    (`self.CreateChild` CollidingSide NewCompClass)
    (else
      (set `self.Real` SetReal)
      (set `self.Stable` SetStable)
      (set `self.Constructed` SetConstructed)
      (`self.ReconstructClassObject`))))

(event `CreateChild`
  (params (AttachingSide :type "ActorComponent Object Reference") (ChildClass :type "Actor Class Reference"))
  (bind _rootsphere (`self.RootSphere`))
  ;[1 1 1] Creating New Compomemt
  (set `self.NewComponentOffset` (0.0 0.0 0.0))
  (`self.SetSideOffset` AttachingSide)
  (if (not (== (`self.NewComponentOffset`) (0.0 0.0 0.0) :`ErrorTolerance` 0.0))
    (bind _returnvalue (`|SpawnActorFromClass` ChildClass (`KismetMathLibrary.MakeTransform` (+ (`self.NewComponentOffset`) (`SceneComponent.K2_GetComponentLocation` _rootsphere)) (`SceneComponent.K2_GetComponentRotation` _rootsphere)) "AdjustIfPossibleButDontSpawnIfColliding" "OverrideRootScale"))
    (`/Engine/EditorBlueprintResources/StandardMacros.IsValid` _returnvalue
      (:`Is Valid`
        (bind _ascomp_parent (cast `/Game/Blueprints/Components/CompParent` _returnvalue))
        (set `self.NewComp` _ascomp_parent))
      (:`Is Not Valid`
        (set `self.NewComp` null)))
    (`self.ReconstructClassObject`)))

(fn `ReconstructClassObject`
  (bind _returnvalue (`KismetMathLibrary.SelectInt` 0 1 (not (`self.Constructed`))))
  (if (`self.Real`)
    (for _array_element (`self.GetComponentsByTag` self "/Script/Engine.StaticMeshComponent" "Basement")
      (`PrimitiveComponent.SetCollisionEnabled` _array_element (`KismetArrayLibrary.Array_Get` (`self.CollisionTypes`) _returnvalue))
      (`PrimitiveComponent.SetMaterial` _array_element 0 (`KismetArrayLibrary.Array_Get` (`self.MaterialTypes`) _returnvalue)))
    (`|ExecutionSequence`
      (:`then_0`
        (`self.RevalidateTrace`))
      (:`then_1`
        (return)))
    (else
      (`self.K2_DestroyActor` self)
      (return))))

(fn `RevalidateTrace`
  (bind _rootsphere (`self.RootSphere`))
  (bind _rootsphere_2 (`self.RootSphere`))
  (bind _rootsphere_3 (`self.RootSphere`))
  (bind _rootsphere_4 (`self.RootSphere`))
  (bind _rootsphere_5 (`self.RootSphere`))
  (bind _rootsphere_6 (`self.RootSphere`))
  (bind _initvalid3 (`self.InitValid3`))
  (bind _initvalid2 (`self.InitValid2`))
  (bind _initvalid4 (`self.InitValid4`))
  (bind _initvalid5 (`self.InitValid5`))
  (bind _initvalid6 (`self.InitValid6`))
  (bind _initvalid1 (`self.InitValid1`))
  (bind _returnvalue (`SceneComponent.K2_GetComponentLocation` _rootsphere_2))
  (bind _returnvalue_2 (`SceneComponent.K2_GetComponentLocation` _rootsphere_3))
  (bind _returnvalue_3 (`SceneComponent.K2_GetComponentLocation` _rootsphere_4))
  (bind _returnvalue_4 (`SceneComponent.K2_GetComponentLocation` _rootsphere_5))
  (bind _returnvalue_5 (`SceneComponent.K2_GetComponentLocation` _rootsphere_6))
  (bind _returnvalue_6 (`SceneComponent.K2_GetComponentLocation` _rootsphere))
  (`|ExecutionSequence`
    (:`then_0`
      (bind _outhit (`KismetSystemLibrary.LineTraceSingleForObjects` :`Start` _returnvalue_3 :`End` (+ _returnvalue_3 (* (`SceneComponent.GetForwardVector` _rootsphere_4) (/ (`self.OffsetValue`) -2.0))) :`ObjectTypes` (`|MakeArray` "ObjectTypeQuery2" :!type "EObjectTypeQuery Enum") :`DrawDebugType` "ForOneFrame"))
      (bind _ascomp_parent (cast `/Game/Blueprints/Components/CompParent` (`.HitActor` (`GameplayStatics.BreakHitResult` _outhit)))
        (:`then`
          (set `self.Neighb3` _ascomp_parent)
          (set `self.CurValid3` (and _initvalid3 false)))
        (:`CastFailed`
          (set `self.Neighb3` null)
          (set `self.CurValid3` (and _initvalid3 true)))))
    (:`then_1`
      (bind _outhit_2 (`KismetSystemLibrary.LineTraceSingleForObjects` :`Start` _returnvalue_4 :`End` (+ _returnvalue_4 (* (`SceneComponent.GetForwardVector` _rootsphere_5) (/ (`self.OffsetValue`) -2.0))) :`ObjectTypes` (`|MakeArray` "ObjectTypeQuery2" :!type "EObjectTypeQuery Enum") :`DrawDebugType` "ForOneFrame"))
      (bind _ascomp_parent_2 (cast `/Game/Blueprints/Components/CompParent` (`.HitActor` (`GameplayStatics.BreakHitResult` _outhit_2)))
        (:`then`
          (set `self.Neighb1` _ascomp_parent_2)
          (set `self.CurValid1` (and _initvalid1 false)))
        (:`CastFailed`
          (set `self.Neighb1` null)
          (set `self.CurValid1` (and _initvalid1 true)))))
    (:`then_2`
      (bind _outhit_3 (`KismetSystemLibrary.LineTraceSingleForObjects` :`Start` _returnvalue_5 :`End` (+ _returnvalue_5 (* (`SceneComponent.GetRightVector` _rootsphere_6) (/ (`self.OffsetValue`) 2.0))) :`ObjectTypes` (`|MakeArray` "ObjectTypeQuery2" :!type "EObjectTypeQuery Enum") :`DrawDebugType` "ForOneFrame"))
      (bind _ascomp_parent_3 (cast `/Game/Blueprints/Components/CompParent` (`.HitActor` (`GameplayStatics.BreakHitResult` _outhit_3)))
        (:`then`
          (set `self.Neighb2` _ascomp_parent_3)
          (set `self.CurValid2` (and _initvalid2 false)))
        (:`CastFailed`
          (set `self.Neighb2` null)
          (set `self.CurValid2` (and _initvalid2 true)))))
    (:`then_3`
      (bind _outhit_4 (`KismetSystemLibrary.LineTraceSingleForObjects` :`Start` _returnvalue :`End` (+ _returnvalue (* (`SceneComponent.GetRightVector` _rootsphere_2) (/ (`self.OffsetValue`) -2.0))) :`ObjectTypes` (`|MakeArray` "ObjectTypeQuery2" :!type "EObjectTypeQuery Enum") :`DrawDebugType` "ForOneFrame"))
      (bind _ascomp_parent_4 (cast `/Game/Blueprints/Components/CompParent` (`.HitActor` (`GameplayStatics.BreakHitResult` _outhit_4)))
        (:`then`
          (set `self.Neighb4` _ascomp_parent_4)
          (set `self.CurValid4` (and _initvalid4 false)))
        (:`CastFailed`
          (set `self.Neighb4` null)
          (set `self.CurValid4` (and _initvalid4 true)))))
    (:`then_4`
      (bind _outhit_5 (`KismetSystemLibrary.LineTraceSingleForObjects` :`Start` _returnvalue_2 :`End` (+ _returnvalue_2 (* (`SceneComponent.GetUpVector` _rootsphere_3) (/ (`self.OffsetValue`) 2.0))) :`ObjectTypes` (`|MakeArray` "ObjectTypeQuery2" :!type "EObjectTypeQuery Enum") :`DrawDebugType` "ForOneFrame"))
      (bind _ascomp_parent_5 (cast `/Game/Blueprints/Components/CompParent` (`.HitActor` (`GameplayStatics.BreakHitResult` _outhit_5)))
        (:`then`
          (set `self.Neighb5` _ascomp_parent_5)
          (set `self.CurValid5` (and _initvalid5 false)))
        (:`CastFailed`
          (set `self.Neighb5` null)
          (set `self.CurValid5` (and _initvalid5 true)))))
    (:`then_5`
      (bind _outhit_6 (`KismetSystemLibrary.LineTraceSingleForObjects` :`Start` _returnvalue_6 :`End` (+ _returnvalue_6 (* (`SceneComponent.GetUpVector` _rootsphere) (/ (`self.OffsetValue`) -2.0))) :`ObjectTypes` (`|MakeArray` "ObjectTypeQuery2" :!type "EObjectTypeQuery Enum") :`DrawDebugType` "ForOneFrame"))
      (bind _ascomp_parent_6 (cast `/Game/Blueprints/Components/CompParent` (`.HitActor` (`GameplayStatics.BreakHitResult` _outhit_6)))
        (:`then`
          (set `self.Neighb6` _ascomp_parent_6)
          (set `self.CurValid6` (and _initvalid6 false)))
        (:`CastFailed`
          (set `self.Neighb6` null)
          (set `self.CurValid6` (and _initvalid6 true)))))))

(fn `SetSideOffset`
  (params (Side :type "ActorComponent Object Reference"))
  (bind _offsetvalue (`self.OffsetValue`))
  (set `self.NewComponentOffset` (`KismetMathLibrary.MakeVector` (* (+ (* (`KismetMathLibrary.Conv_BoolToInt` (and (`self.CurValid1`) (== Side (`self.Side1`)))) -1) (`KismetMathLibrary.Conv_BoolToInt` (and (`self.CurValid3`) (== Side (`self.Side3`))))) _offsetvalue) (* (+ (`KismetMathLibrary.Conv_BoolToInt` (and (`self.CurValid2`) (== Side (`self.Side2`)))) (* (`KismetMathLibrary.Conv_BoolToInt` (and (`self.CurValid4`) (== Side (`self.Side4`)))) -1)) _offsetvalue) (* (+ (`KismetMathLibrary.Conv_BoolToInt` (and (`self.CurValid5`) (== Side (`self.Side5`)))) (* (`KismetMathLibrary.Conv_BoolToInt` (and (`self.CurValid6`) (== Side (`self.Side6`)))) -1)) _offsetvalue)))
  (return))

(fn `UserConstructionScript`
  (`self.ReconstructClassObject`))