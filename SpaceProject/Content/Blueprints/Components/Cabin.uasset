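; Cabin is a ship component Blueprint that acts as the root cabin and creates the ship's controller.
; Construction runs the parent script, then marks the cabin as connected and sets itself as its own RootCabin.
; SpawnController spawns a ShipController at the cabin's transform regardless of collision, calls SpawnDefaultController on it, and links cabin and controller to each other.
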(fn `SpawnController`
  (bind _returnvalue (`|SpawnActorFromClass` "/Game/Blueprints/Components/ShipController.ShipController_C" (`self.GetTransform` self) "AlwaysSpawn" "OverrideRootScale"))
  (bind _output_get (set `self.Controller` _returnvalue))
  (`Pawn.SpawnDefaultController` _output_get)
  (set `/Game/Blueprints/Components/ShipController.Cabin` self _output_get))

(fn `UserConstructionScript`
  (`parent.UserConstructionScript`)
  (set `self.IsConnectedToCabin` true)
  (set `self.RootCabin` self))