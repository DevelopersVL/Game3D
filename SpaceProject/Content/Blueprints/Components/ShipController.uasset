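; Ship controller that flies a physics-driven ship from player input, with movement and rotation on all three axes.
; Each input axis adds linear velocity (scaled by FlyingSpeed) or angular velocity to the Cabin's Basement along its own forward, right or up vector, without delta-time scaling.
; Pressing G unpossesses the current pawn, possesses the MyPawn1 actors found in the level in turn, and switches the view target.
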(event `InputAxis|ImpulseForward`
  (params (AxisValue :type "Float (single-precision)"))
  (bind _basement (`/Game/Blueprints/Components/CompParent.Basement` (`self.Cabin`)))
  ;[1 1 1] Movement
  (`PrimitiveComponent.SetPhysicsLinearVelocity` _basement (* (`SceneComponent.GetForwardVector` _basement) (* (`self.Flying Speed`) AxisValue)) true "None"))

(event `InputAxis|LookUp`
  (params (AxisValue :type "Float (single-precision)"))
  (bind _basement (`/Game/Blueprints/Components/CompParent.Basement` (`self.Cabin`)))
  ;[1 1 1] Rotation
  (`PrimitiveComponent.SetPhysicsAngularVelocity` _basement (* (`SceneComponent.GetRightVector` _basement) AxisValue) true "None"))

(event `Key|G`
  (params (Key :type "Key Structure" :default "AnyKey"))
  (bind _returnvalue (`GameplayStatics.GetPlayerController` 0))
  (:`Pressed`
    (`Controller.UnPossess` _returnvalue)
    (bind _outactors (`GameplayStatics.GetAllActorsOfClass` "/Game/Blueprints/MyPawn1.MyPawn1_C"))
    (for _array_element _outactors
      (`Controller.Possess` _returnvalue _array_element))
    (`PlayerController.SetViewTargetWithBlend` _returnvalue _array_element 0.0 "VTBlend_Linear" 0.0 false)))

(event `InputAxis|Jump/FlyUp`
  (params (AxisValue :type "Float (single-precision)"))
  (bind _basement (`/Game/Blueprints/Components/CompParent.Basement` (`self.Cabin`)))
  ;[1 1 1] Movement
  (`PrimitiveComponent.SetPhysicsLinearVelocity` _basement (* (`SceneComponent.GetUpVector` _basement) (* (`self.Flying Speed`) AxisValue)) true "None"))

(event `InputAxis|Turn`
  (params (AxisValue :type "Float (single-precision)"))
  (bind _basement (`/Game/Blueprints/Components/CompParent.Basement` (`self.Cabin`)))
  ;[1 1 1] Rotation
  (`PrimitiveComponent.SetPhysicsAngularVelocity` _basement (* (`SceneComponent.GetUpVector` _basement) AxisValue) true "None"))

(event `InputAxis|Crouch/FlyDown`
  (params (AxisValue :type "Float (single-precision)"))
  (bind _basement (`/Game/Blueprints/Components/CompParent.Basement` (`self.Cabin`)))
  ;[1 1 1] Movement
  (`PrimitiveComponent.SetPhysicsLinearVelocity` _basement (* (`SceneComponent.GetUpVector` _basement) (* (`self.Flying Speed`) AxisValue)) true "None"))

(event `InputAxis|Roll`
  (params (AxisValue :type "Float (single-precision)"))
  (bind _basement (`/Game/Blueprints/Components/CompParent.Basement` (`self.Cabin`)))
  ;[1 1 1] Rotation
  (`PrimitiveComponent.SetPhysicsAngularVelocity` _basement (* (`SceneComponent.GetForwardVector` _basement) AxisValue) true "None"))

(event `InputAxis|ImpulseRight`
  (params (AxisValue :type "Float (single-precision)"))
  (bind _basement (`/Game/Blueprints/Components/CompParent.Basement` (`self.Cabin`)))
  ;[1 1 1] Movement
  (`PrimitiveComponent.SetPhysicsLinearVelocity` _basement (* (`SceneComponent.GetRightVector` _basement) (* (`self.Flying Speed`) AxisValue)) true "None"))

(fn `UserConstructionScript`)