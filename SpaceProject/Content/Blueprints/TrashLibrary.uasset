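; TrashLibrary is a Blueprint helper library with one function, RotatorAdd, which offsets a rotator by separate roll, pitch and yaw amounts.
; It adds each component directly, then loops until all three lie in an asymmetric -160 to 200 degree range, rather than the usual -180 to 180.
; Each pass converts the bound comparisons to integers to shift out-of-range axes by a full turn without branching.
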(fn RotatorAdd
  (params (Rotator :type Rotator) (Roll :type Float%20%28single-precision%29) (Pitch :type Float%20%28single-precision%29) (Yaw :type Float%20%28single-precision%29))
  (bind (_roll _pitch _yaw) (Math|Rotator|BreakRotator Rotator))
  (LocalVariables|SetMyRotator (Math|Rotator|MakeRotator (+ _roll Roll) (+ _pitch Pitch) (+ _yaw Yaw)))
  (while (Math|Boolean|ORBoolean (>= (.Roll (Math|Rotator|BreakRotator (LocalVariables|GetMyRotator))) 2e+02) (< (.Roll (Math|Rotator|BreakRotator (LocalVariables|GetMyRotator))) -1.6e+02) (>= (.Pitch (Math|Rotator|BreakRotator (LocalVariables|GetMyRotator))) 2e+02) (< (.Pitch (Math|Rotator|BreakRotator (LocalVariables|GetMyRotator))) -1.6e+02) (>= (.Yaw (Math|Rotator|BreakRotator (LocalVariables|GetMyRotator))) 2e+02) (< (.Yaw (Math|Rotator|BreakRotator (LocalVariables|GetMyRotator))) -1.6e+02))
    (LocalVariables|SetMyRotator (Math|Rotator|MakeRotator (+ (.Roll (Math|Rotator|BreakRotator (LocalVariables|GetMyRotator))) (* (+ (* -1 (Math|Conversions|ToInteger(Boolean) (>= (.Roll (Math|Rotator|BreakRotator (LocalVariables|GetMyRotator))) 2e+02))) (Math|Conversions|ToInteger(Boolean) (< (.Roll (Math|Rotator|BreakRotator (LocalVariables|GetMyRotator))) -1.6e+02))) 3.6e+02)) (+ (.Pitch (Math|Rotator|BreakRotator (LocalVariables|GetMyRotator))) (* (+ (* -1 (Math|Conversions|ToInteger(Boolean) (>= (.Pitch (Math|Rotator|BreakRotator (LocalVariables|GetMyRotator))) 2e+02))) (Math|Conversions|ToInteger(Boolean) (< (.Pitch (Math|Rotator|BreakRotator (LocalVariables|GetMyRotator))) -1.6e+02))) 3.6e+02)) (+ (.Yaw (Math|Rotator|BreakRotator (LocalVariables|GetMyRotator))) (* (+ (* -1 (Math|Conversions|ToInteger(Boolean) (>= (.Yaw (Math|Rotator|BreakRotator (LocalVariables|GetMyRotator))) 2e+02))) (Math|Conversions|ToInteger(Boolean) (< (.Yaw (Math|Rotator|BreakRotator (LocalVariables|GetMyRotator))) -1.6e+02))) 3.6e+02)))))
  (return (LocalVariables|GetMyRotator)))